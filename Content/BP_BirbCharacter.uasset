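; Bird character Blueprint for a Jump Birb game that animates the bird falling off screen on game over.
; On BeginPlay it binds to the BP_JumpBirbGameMode game state change event.
; At Game Over it caches its location and plays a timeline whose vector track offsets the actor from that point.
; Each timeline update also zeroes the capsule's physics linear velocity to stop continuous falling.
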(event Custom|AnimateFallingOffScreen
  (params (GameState :type EGameState%20Enum :default "Menu"))
  ;[1 1 1] Animate falling off screen on game over
  (switch Utilities|FlowControl|Switch|SwitchonEGameState GameState
    (:GameOver
      (bind _output_get (Variables|Default|SetLocationAtGameOver (Transformation|GetActorLocation)))
      (bind _vector (Timeline|FallingAnimation PlayFromStart)
        (:Update
          (Transformation|SetActorLocation (+ _output_get _vector) false false)
          (Physics|SetPhysicsLinearVelocity (Variables|Default|GetCapsuleComponent) "0, 0, 0" false "None") ; Stops the character from continuously falling
        )))))

(event EventBeginPlay
  (|CallParentFunction)
  (bind _asbp_jump_birb_game_mode (Utilities|Casting|CastToBP_JumpBirbGameMode (Game|GetGameMode)))
  (EventDispatchers|BindEventtoOnGameStateChange _asbp_jump_birb_game_mode (EventDispatchers|CreateEvent :!event Custom|AnimateFallingOffScreen)))

(fn ConstructionScript)