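; HUD for the JumpBirb game that shows and hides UI screens as the game state changes.
; On BeginPlay it enables mouse input, creates the main menu and a hidden game widget, then binds to the game mode's state-change event.
; A state switch toggles those persistent widgets' visibility and creates the jump-start and game-over screens on demand, removing jump-start when play begins.
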(event Custom|OnGameStateChange
  (params (GameState :type EGameState%20Enum :default "Menu"))
  (switch Utilities|FlowControl|Switch|SwitchonEGameState GameState
    (:Menu
      (Widget|SetVisibility (Variables|Default|GetGame_Ref) "Collapsed")
      (Widget|SetVisibility (Variables|Default|GetMainMenu_Ref) "Visible"))
    (:Setup
      (Widget|SetVisibility (Variables|Default|GetMainMenu_Ref) "Collapsed")
      (bind _returnvalue (UserInterface|CreateWidget "/Game/UI/UI_JumpStart.UI_JumpStart_C"))
      (UserInterface|Viewport|AddtoViewport _returnvalue 0))
    (:StartGame
      (Widget|RemovefromParent _returnvalue)
      (CallFunction|ToggleWidget (Variables|Default|GetGame_Ref)))
    (:GameOver
      (CallFunction|ToggleWidget (Variables|Default|GetGame_Ref))
      (bind _returnvalue_2 (UserInterface|CreateWidget "/Game/UI/UI_GameOver.UI_GameOver_C"))
      (UserInterface|Viewport|AddtoViewport _returnvalue_2 0))))

(event EventBeginPlay
  (CallFunction|SetUpUI)
  (bind _asbp_jump_birb_game_mode (Utilities|Casting|CastToBP_JumpBirbGameMode (Game|GetGameMode)))
  (bind _output_get (Variables|Default|SetGameMode_Ref _asbp_jump_birb_game_mode))
  (EventDispatchers|BindEventtoOnGameStateChange _output_get (EventDispatchers|CreateEvent :!event Custom|OnGameStateChange)))

(fn ConstructionScript)

(fn SetUpUI
  (bind _returnvalue (Game|GetPlayerController 0))
  (Variables|/Script/Engine.PlayerController|SetbShowMouseCursor _returnvalue true)
  (Input|SetInputModeGameandUI _returnvalue 0 "DoNotLock" false false)
  (bind _returnvalue_2 (UserInterface|CreateWidget "/Game/UI/UI_MainMenu.UI_MainMenu_C"))
  (bind _output_get (Variables|Default|SetMainMenu_Ref _returnvalue_2))
  (UserInterface|Viewport|AddtoViewport _output_get 0)
  (bind _returnvalue_3 (UserInterface|CreateWidget "/Game/UI/UI_Game.UI_Game_C"))
  (bind _output_get_2 (Variables|Default|SetGame_Ref _returnvalue_3))
  (Widget|SetVisibility _output_get_2 "Collapsed")
  (UserInterface|Viewport|AddtoViewport _output_get_2 0))

(fn ToggleWidget
  (params (Widget :type User%20Widget%20Object%20Reference))
  (if (Widget|IsVisible Widget)
    (Widget|SetVisibility Widget "Collapsed")
    (else
      (Widget|SetVisibility Widget "Visible"))))